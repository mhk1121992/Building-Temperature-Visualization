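; Building floor actor assembled from many mesh components, including main structure, roof, stairs, cubes and CubeGrid tool outputs.
; SetFloorMaterial applies one material to the first slot of all the listed components, restyling them together.
; A stored Temperature value has a simple setter and getter, with no link to the material in this Blueprint.
; The event graph and construction script are empty, so changes come only through function calls.
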(event `self.ReceiveBeginPlay`)

(fn `GetFloorTemperature`
  (returns (OutTemperature :type "Float (double-precision)"))
  (return (`self.Temperature`)))

(fn `SetFloorMaterial`
  (params (Material :type "MaterialInterface Object Reference"))
  (`PrimitiveComponent.SetMaterial` (`self.Cube2`) 0 Material)
  (`PrimitiveComponent.SetMaterial` (`self.CubeGridToolOutput_CAA0C212`) 0 Material)
  (`PrimitiveComponent.SetMaterial` (`self.Cube`) 0 Material)
  (`PrimitiveComponent.SetMaterial` (`self.Stairs_A099560F`) 0 Material)
  (`PrimitiveComponent.SetMaterial` (`self.MainStructure`) 0 Material)
  (`PrimitiveComponent.SetMaterial` (`self.Roof`) 0 Material)
  (`PrimitiveComponent.SetMaterial` (`self.CubeGridToolOutput_CAA0C214`) 0 Material)
  (`PrimitiveComponent.SetMaterial` (`self.CubeGridToolOutput_CAA0C213`) 0 Material)
  (`PrimitiveComponent.SetMaterial` (`self.Cube1`) 0 Material)
  (`PrimitiveComponent.SetMaterial` (`self.Cube9`) 0 Material)
  (`PrimitiveComponent.SetMaterial` (`self.Cube8`) 0 Material)
  (`PrimitiveComponent.SetMaterial` (`self.Cube7`) 0 Material)
  (`PrimitiveComponent.SetMaterial` (`self.Cube4`) 0 Material)
  (`PrimitiveComponent.SetMaterial` (`self.Cube3`) 0 Material)
  (`PrimitiveComponent.SetMaterial` (`self.Cube5`) 0 Material)
  (`PrimitiveComponent.SetMaterial` (`self.Cube6`) 0 Material))

(fn `SetFloorTemperature`
  (params (InTemperature :type "Float (double-precision)"))
  (set `self.Temperature` InTemperature))

(fn `UserConstructionScript`)
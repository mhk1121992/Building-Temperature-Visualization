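; Actor in the building configurator GUI that carries a text widget, apparently for showing floor data outside the building.
; On BeginPlay it sets the root to a fixed world rotation with a -90 degree turn.
; A looping timer that turns the widget toward the player camera is present but never started, and is marked for deletion.
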(event `self.ReceiveBeginPlay`
  (`SceneComponent.K2_SetWorldRotation` (`self.DefaultSceneRoot`) (struct :`Yaw` -90.0) false false))

(event `StartTimer`
  ;[0.5208 0.1807 0.16] To be deleted - Widget faces the camera - Update widget rotation every 0.2 second
  (`KismetSystemLibrary.K2_SetTimerDelegate` (delegate `UpdateRotation`) 0.2 true))

(event `UpdateRotation`
  (bind _textwidget (`self.TextWidget`))
  ;[0.5208 0.1807 0.16] To be deleted - Widget faces the camera - Update widget rotation every 0.2 second
  (`SceneComponent.K2_SetWorldRotation` _textwidget (`KismetMathLibrary.FindLookAtRotation` (`SceneComponent.K2_GetComponentLocation` _textwidget) (`PlayerCameraManager.GetCameraLocation` (`GameplayStatics.GetPlayerCameraManager` 0))) false false))

(fn `UserConstructionScript`)
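; InsideFloorDataViz2_BP is a building configurator GUI actor, apparently for floor data visualization, that keeps its widget facing the player camera.
; BeginPlay starts a looping 0.2-second timer instead of using Tick.
; Each timer call rotates the scene root toward the camera location with a look-at rotation.
; The billboard logic is marked for deletion, and a fixed-rotation node is left unconnected.
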(event `self.ReceiveBeginPlay`
  (`self.StartTimer`))

(event `StartTimer`
  ;[0.5208 0.1807 0.16] To be deleted - Widget faces the camera - Update widget rotation every 0.2 second
  (`KismetSystemLibrary.K2_SetTimerDelegate` (delegate `UpdateRotation`) 0.2 true))

(event `UpdateRotation`
  (bind _defaultsceneroot (`self.DefaultSceneRoot`))
  ;[0.5208 0.1807 0.16] To be deleted - Widget faces the camera - Update widget rotation every 0.2 second
  (`SceneComponent.K2_SetWorldRotation` _defaultsceneroot (`KismetMathLibrary.FindLookAtRotation` (`SceneComponent.K2_GetComponentLocation` _defaultsceneroot) (`PlayerCameraManager.GetCameraLocation` (`GameplayStatics.GetPlayerCameraManager` 0))) false false))

(fn `UserConstructionScript`)
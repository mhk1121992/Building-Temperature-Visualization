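; Building config actor that visualizes per-floor temperatures and creates the main UI on BeginPlay.
; For each floor, it looks up temperature by the number parsed from the display name, then spawns exterior and interior world-space widget actors showing name and temperature.
; An HSV hue mapped from temperature tints the exterior text and its cube via a dynamic material.
; Widgets are mapped by floor, but refresh updates only the last-spawned pair.
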(event `self.ReceiveBeginPlay`
  (`|ExecutionSequence`
    (:`then_0`
      ;[0 0 0] Spawning Main UI
      (bind _returnvalue (`|CreateWidget` "/Game/Blueprints/Main_GUI/Main_UI.Main_UI_C"))
      (bind _output_get (set `self.MainUI_Ref` _returnvalue))
      (`UserWidget.AddToViewport` _output_get 0))
    (:`then_1`
      (for _array_element (`self.BuildingFloors`)
        (`|ExecutionSequence`
          (:`then_0`
            ;[0 0 0] Calling them in sequence is necessary because the below function relies on the "Spawn Exterior Widget" Macro
            ;;[0 0 0] Spwan a widget outside every floor
            (`self.SpawnExteriorWidget` _array_element _array_element))
          (:`then_1`
            ;;[0 0 0] Spawn a widget inside every floor
            (`self.SpawnInteriorWidget`)))))))

(fn `GetColorByTemperature`
  (params (TemperatureIn :type "Float (double-precision)"))
  (returns (ReturnValue :type "LinearColor Structure"))
  (locals (LinearColor :type "LinearColor Structure" :default (struct)))
  (bind _linearcolor (`local.LinearColor`))
  (`KismetMathLibrary.LinearColor_SetFromHSV` _linearcolor (`KismetMathLibrary.MapRangeClamped` TemperatureIn -100.0 100.0 0.0 359.0) 1.0 1.0)
  (return _linearcolor))

(fn `GetFloorNumberAndTemperature`
  (returns (SetTempByFloorNumber :type "Map of String to Float (double-precision)"))
  (return (`self.SetTempByFloorNumber`)))

(fn `GetFloors`
  (returns (BuildingFloors :type "Array of Actor Object Reference"))
  (return (`self.BuildingFloors`)))

(fn `RefreshFloorWidgets`
  (params (Floor :type "/Game/Blueprints/Building/Floor Object Reference"))
  (locals (Temp :type "Float (double-precision)" :default 0.0))
  (bind _outtemperature (`/Game/Blueprints/Building/Floor.GetFloorTemperature` Floor))
  (bind _output_get (set `local.Temp` _outtemperature))
  (bind _returnvalue (`KismetTextLibrary.Conv_StringToText` (`KismetStringLibrary.Concat_StrStr` (`KismetStringLibrary.Conv_DoubleToString` _output_get) "°")))
  ;[0 0 0] Set text of the exterior widget
  (set `TextBlock.Text` _returnvalue (`/Game/Blueprints/BuildingConfig/GUI/OutsideFloorDataViz_UI.TemperatureText` (cast `/Game/Blueprints/BuildingConfig/GUI/OutsideFloorDataViz_UI` (`WidgetComponent.GetUserWidgetObject` (`/Game/Blueprints/BuildingConfig/GUI/OutsideFloorDataViz_BP.TextWidget` (`self.OutsideFloorDataVizBP_Ref`))) :!pure true)))
  ;[0 0 0] Set text of the interior widget
  (set `TextBlock.Text` _returnvalue (`/Game/Blueprints/BuildingConfig/GUI/InsideFloorDataViz_UI.TemperatureText` (cast `/Game/Blueprints/BuildingConfig/GUI/InsideFloorDataViz_UI` (`WidgetComponent.GetUserWidgetObject` (`/Game/Blueprints/BuildingConfig/GUI/InsideFloorDataViz2_BP.TextWidget` (`self.InsideFloorDataVizBP_Ref`))) :!pure true))))

(fn `Set Current Floor Name In Exterior Widget`
  (`TextRenderComponent.K2_SetText` (`/Game/Blueprints/BuildingConfig/GUI/OutsideFloorDataViz_BP.FloorName` (`self.OutsideFloorDataVizBP_Ref`)) (`KismetTextLibrary.Conv_StringToText` (`KismetSystemLibrary.GetDisplayName` (`self.CurrentFloor`)))))

(fn `Set Current Floor Name In Interior  Widget`
  (`TextRenderComponent.K2_SetText` (`/Game/Blueprints/BuildingConfig/GUI/InsideFloorDataViz2_BP.FloorName` (`self.InsideFloorDataVizBP_Ref`)) (`KismetTextLibrary.Conv_StringToText` (`KismetSystemLibrary.GetDisplayName` (`self.CurrentFloor`)))))

(fn `SetExteriorWidgetColorAndMat`
  (params (ColorIn :type "LinearColor Structure") (MaterialIn :type "MaterialInterface Object Reference"))
  (`TextBlock.SetColorAndOpacity` (`self.OutsideTemperatureText`) (make `SlateColor` ColorIn))
  (`PrimitiveComponent.SetMaterial` (`/Game/Blueprints/BuildingConfig/GUI/OutsideFloorDataViz_BP.Cube` (`self.OutsideFloorDataVizBP_Ref`)) 0 MaterialIn))

(fn `SetFloorNumberAndTemperature`
  (params (InFloorNumber :type "String (by ref)") (InFloorTemp :type "Float (double-precision) (by ref)"))
  (`BlueprintMapLibrary.Map_Add` (`self.SetTempByFloorNumber`) InFloorNumber InFloorTemp))

(fn `SpawnInteriorWidget`
  (bind _returnvalue (`|SpawnActorFromClass` "/Game/Blueprints/BuildingConfig/GUI/InsideFloorDataViz2_BP.InsideFloorDataViz2_BP_C" (`KismetMathLibrary.MakeTransform` (`SceneComponent.K2_GetComponentLocation` (`/Game/Blueprints/Building/Floor.RoomWidgetSpawnPoint_Sphere` (`self.CurrentFloor`)))) "Undefined" "OverrideRootScale" null null))
  (bind _output_get (set `self.InsideFloorDataVizBP_Ref` _returnvalue))
  (bind _output_get_2 (set `self.InsideTemperature Text` (`/Game/Blueprints/BuildingConfig/GUI/InsideFloorDataViz_UI.TemperatureText` (cast `/Game/Blueprints/BuildingConfig/GUI/InsideFloorDataViz_UI` (`WidgetComponent.GetUserWidgetObject` (`/Game/Blueprints/BuildingConfig/GUI/InsideFloorDataViz2_BP.TextWidget` _output_get)) :!pure true))))
  (set `TextBlock.Text` (`KismetTextLibrary.Conv_StringToText` (`KismetStringLibrary.Concat_StrStr` (`KismetStringLibrary.Conv_DoubleToString` (`self.CurrentFloorTemperature`)) "°")) _output_get_2)
  ;[0 0 0] Save floor BP and corresponding interior widget actor to a Map
  (`BlueprintMapLibrary.Map_Add` (`self.FloorAndCorrespondingInteriorWidgetActor`) (`self.CurrentFloor`) (`self.InsideFloorDataVizBP_Ref`))
  (`self.Set Current Floor Name In Interior  Widget`))

(fn `UserConstructionScript`)